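; Test-map Blueprint that lays out copies of a static mesh along a spline as hierarchical instances, built entirely in the Construction Script.
; A helper derives the copy count from mesh, spline and extra spacing, then the spline length is split evenly by that count.
; Each segment's midpoint yields a local-space, spline-aligned, unit-scale transform, and a second helper adds these to the HISM.
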(event `self.ReceiveBeginPlay`)

(fn `UserConstructionScript`
  (locals (Transforms :type "Array of Transform Structure"))
  (bind _spline (`self.Spline`))
  (bind _count (`/Game/procedural_building/BPL_ProceduralBuilding.PB_CopyCountAlongSpline` (`self.Spline`) (`self.StaticMesh`) (`self.SpacedByMeshSizeAdditionSpacing`)))
  (for _index (range _count)
    (`KismetSystemLibrary.PrintString` "")
    (bind _returnvalue (* (+ (`KismetMathLibrary.Conv_IntToDouble` _index) 0.5) (/ (`SplineComponent.GetSplineLength` (`self.Spline`)) (`KismetMathLibrary.Conv_IntToDouble` _count))))
    (`KismetArrayLibrary.Array_Add` (`local.Transforms`) (`KismetMathLibrary.MakeTransform` (`SplineComponent.GetLocationAtDistanceAlongSpline` _spline _returnvalue "Local") (`SplineComponent.GetRotationAtDistanceAlongSpline` _spline _returnvalue "Local"))))
  (`StaticMeshComponent.SetStaticMesh` (`self.HierarchicalInstancedStaticMesh`) (`self.StaticMesh`))
  (`/Game/procedural_building/BPL_ProceduralBuilding.PB_AddInstancesToHISM` (`self.HierarchicalInstancedStaticMesh`) (`local.Transforms`)))
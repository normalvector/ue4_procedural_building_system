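; Test Blueprint for PBSelectNear that builds a grid of instanced meshes in its construction script.
; A probability split marks about one percent of items, which are jittered upward and added to the glowing HISM.
; PBSelectNear divides the rest by distance to those marked items.
; Near neighbours get a smaller vertical jitter in the red HISM, while the others stay unmoved in the black one.
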(fn `UserConstructionScript`
  ;[1 1 1] Select the items we're marking
  (bind (_transformsunselected _transformsselected) (`/Game/procedural_building/BPL_ProceduralBuilding.PB_SplitWithProbability` (`/Game/procedural_building/BPL_ProceduralBuilding.PB_LinearArray` (`/Game/procedural_building/BPL_ProceduralBuilding.PB_DefaultItem`) (30.0 30.0 1.0) (`/Game/procedural_building/BPL_ProceduralBuilding.PB_StaticMeshItemSize` (`StaticMeshComponent.StaticMesh` (`self.HierarchicalInstancedStaticMeshBlack`))) (0.0 0.0 0.0) (0.0 0.0 0.0)) 0.01 (`self.RandomStream`)))
  (bind (_selected _unselected) (`/Game/procedural_building/BPL_ProceduralBuilding.PB_SelectNear` _transformsunselected _transformsselected 500.0))
  ;[1 1 1] Jitter neighbours
  (bind _transforms (`/Game/procedural_building/BPL_ProceduralBuilding.PB_JitterPosition` _selected (0.0 0.0 50.0) (`self.RandomStream`) 0.0))
  (bind _transforms_2 (`/Game/procedural_building/BPL_ProceduralBuilding.PB_JitterPosition` _transformsselected (0.0 0.0 200.0) (struct) 0.5))
  (`/Game/procedural_building/BPL_ProceduralBuilding.PB_AddInstancesToHISM` (`self.HierarchicalInstancedStaticMeshGlowing`) _transforms_2)
  (`/Game/procedural_building/BPL_ProceduralBuilding.PB_AddInstancesToHISM` (`self.HierarchicalInstancedStaticMeshRed`) _transforms)
  (`/Game/procedural_building/BPL_ProceduralBuilding.PB_AddInstancesToHISM` (`self.HierarchicalInstancedStaticMeshBlack`) _unselected))
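; BP_LinearArrayWithRangeDecay is a test-map actor that builds a line of red bevelled cubes thinned by random decay from both ends.
; The construction script uses PB functions to create a ten-item linear array along Z, spaced by the mesh's size.
; PBRangeDecay filters the transforms using decay chance, start and end ranges and a random stream.
; The resulting transforms become instances on a HierarchicalInstancedStaticMesh, with no active runtime logic.
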(fn `UserConstructionScript`
  (bind _hierarchicalinstancedstaticmesh (`self.HierarchicalInstancedStaticMesh`))
  (`StaticMeshComponent.SetStaticMesh` _hierarchicalinstancedstaticmesh "/Game/basic_geometry/BevelledUnitCube.BevelledUnitCube")
  (`PrimitiveComponent.SetMaterial` _hierarchicalinstancedstaticmesh 0 "/Game/simple_pbr_material/MI_ShinyRed.MI_ShinyRed")
  (bind _transforms (`/Game/procedural_building/BPL_ProceduralBuilding.PB_RangeDecay` (`/Game/procedural_building/BPL_ProceduralBuilding.PB_LinearArray` (`/Game/procedural_building/BPL_ProceduralBuilding.PB_DefaultItem`) (1.0 1.0 10.0) (`/Game/procedural_building/BPL_ProceduralBuilding.PB_StaticMeshItemSize` (`StaticMeshComponent.StaticMesh` (`self.HierarchicalInstancedStaticMesh`)))) (`self.DecayChance`) (`self.DecayFromStart`) (`self.DecayFromEnd`) (`self.RandomStream`)))
  (`/Game/procedural_building/BPL_ProceduralBuilding.PB_AddInstancesToHISM` (`self.HierarchicalInstancedStaticMesh`) _transforms))
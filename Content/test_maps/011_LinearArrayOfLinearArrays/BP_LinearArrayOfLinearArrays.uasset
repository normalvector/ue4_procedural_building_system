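; Test Blueprint that builds a procedural grid of instanced meshes by nesting one linear array inside another.
; The construction script starts from a single default item, arrays it along Y, then feeds that row into a second array along Z.
; Both passes derive item size from the HISM's static mesh and add spacing, positional stepping and rotational stepping.
; The resulting transforms are added as instances to the HierarchicalInstancedStaticMesh component.
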(fn `UserConstructionScript`
  ;[1 1 1] Create the instanced meshes
  (`/Game/procedural_building/BPL_ProceduralBuilding.PB_AddInstancesToHISM` (`self.HierarchicalInstancedStaticMesh`) (`/Game/procedural_building/BPL_ProceduralBuilding.PB_LinearArray` (`/Game/procedural_building/BPL_ProceduralBuilding.PB_LinearArray` (`/Game/procedural_building/BPL_ProceduralBuilding.PB_DefaultItem`) (1.0 25.0 1.0) (`/Game/procedural_building/BPL_ProceduralBuilding.PB_StaticMeshItemSize` (`StaticMeshComponent.StaticMesh` (`self.HierarchicalInstancedStaticMesh`))) (0.0 50.0 0.0) (0.0 0.0 0.0) (0.0 0.0 10.0) (0.0 0.0 0.0) (struct) (struct :`Roll` 10.0)) (1.0 1.0 25.0) (`/Game/procedural_building/BPL_ProceduralBuilding.PB_StaticMeshItemSize` (`StaticMeshComponent.StaticMesh` (`self.HierarchicalInstancedStaticMesh`))) (0.0 0.0 50.0) (0.0 0.0 0.0) (0.0 0.0 10.0) (0.0 10.0 0.0) (struct) (struct) (struct :`Roll` 10.0))))
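; Test Blueprint that procedurally builds a flat grid of mixed cube and sphere instances in its construction script.
; A linear array spaced by the cube mesh's size, with a brick offset, generates the transforms, which are then jittered vertically.
; A seeded probability split sends about a quarter of them to the sphere HISM and the rest to the cube HISM.
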(fn `UserConstructionScript`
  (bind _transforms (`/Game/procedural_building/BPL_ProceduralBuilding.PB_JitterPosition` (`/Game/procedural_building/BPL_ProceduralBuilding.PB_LinearArray` (`/Game/procedural_building/BPL_ProceduralBuilding.PB_DefaultItem`) (10.0 10.0 1.0) (`/Game/procedural_building/BPL_ProceduralBuilding.PB_StaticMeshItemSize` (`StaticMeshComponent.StaticMesh` (`self.HISMCube`))) (0.0 0.0 0.0) (0.0 0.0 0.0) (0.0 0.0 0.0) (0.0 0.0 0.0) (struct) (struct) (struct) (0.0 50.0 0.0) (0.0 0.0 0.0) (0.0 0.0 0.0)) (0.0 0.0 5.0) (`self.RandomStream`)))
  (bind (_transformsunselected _transformsselected) (`/Game/procedural_building/BPL_ProceduralBuilding.PB_SplitWithProbability` _transforms 0.25 (`self.RandomStream`)))
  (`/Game/procedural_building/BPL_ProceduralBuilding.PB_AddInstancesToHISM` (`self.HISMCube`) _transformsunselected)
  (`/Game/procedural_building/BPL_ProceduralBuilding.PB_AddInstancesToHISM` (`self.HISMSphere`) _transformsselected))
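; BP_RotateAroundAnyPoint is a test actor that spins a Cube around an arbitrary pivot point marked by a Cylinder.
; The construction script moves the Cylinder to the RotationPoint variable.
; On BeginPlay a looping timeline drives a yaw value into BuildRotationAroundPoint, using the Cylinder's relative location as pivot.
; The resulting transform is applied as the Cube's relative transform each update.
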(event `self.ReceiveBeginPlay`
  (bind (_direction _rotation) (`Timeline|Timeline_0` :!label _label)
    (:`Update`
      (bind _transform (`/Game/procedural_building/BPL_ProceduralBuilding.BP_BuildRotationAroundPoint` (`KismetMathLibrary.MakeVector` 0.0) (`SceneComponent.RelativeLocation` (`self.Cylinder`)) (`KismetMathLibrary.MakeRotator` 0.0 0.0 _rotation)))
      (`SceneComponent.K2_SetRelativeTransform` (`self.Cube`) _transform false false))
    (:`Finished`
      (`KismetSystemLibrary.Delay` 0.0)
      (goto _label :!via `PlayFromStart`))))

(fn `UserConstructionScript`
  (`SceneComponent.K2_SetRelativeLocation` (`self.Cylinder`) (`self.RotationPoint`) false false))
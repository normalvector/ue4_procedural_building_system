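; Demo actor that procedurally builds a linear array of mesh clones as a Hierarchical Instanced Static Mesh in its Construction Script.
; It applies the mesh and materials, then generates stepped, rotated transforms spaced by the mesh's size using PB helper functions.
; Seeded probability splits delete some items and jitter the position and rotation of others.
; The surviving and jittered transforms are rejoined and added as instances.
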(fn `UserConstructionScript`
  ;[1 1 1] Set mesh and materials on hierarchial instanced static mesh
  (`StaticMeshComponent.SetStaticMesh` (`self.HierarchicalInstancedStaticMesh`) (`self.StaticMesh`))
  (for (_array_element _array_index) (`self.Materials`)
    (`PrimitiveComponent.SetMaterial` (`self.HierarchicalInstancedStaticMesh`) _array_index _array_element))
  ;[1 1 1] Delete some items based on chance
  (bind _transformsunselected (`/Game/procedural_building/BPL_ProceduralBuilding.PB_SplitWithProbability` (`/Game/procedural_building/BPL_ProceduralBuilding.PB_LinearArray` (`/Game/procedural_building/BPL_ProceduralBuilding.PB_DefaultItem`) (`self.ItemCount`) (`/Game/procedural_building/BPL_ProceduralBuilding.PB_StaticMeshItemSize` (`StaticMeshComponent.StaticMesh` (`self.HierarchicalInstancedStaticMesh`))) (`self.ItemSpacing`) (`self.SteppingX`) (`self.SteppingY`) (`self.SteppingZ`) (`self.RotationSteppingX`) (`self.RotationSteppingY`) (`self.RotationSteppingZ`)) (`self.DeleteChance`) (`self.RandomStream`)))
  ;[1 1 1] Jitter transforms based on probability
  (bind (_transformsunselected_2 _transformsselected) (`/Game/procedural_building/BPL_ProceduralBuilding.PB_SplitWithProbability` _transformsunselected (`self.JitterChance`) (`self.RandomStream`)))
  (bind _transforms (`/Game/procedural_building/BPL_ProceduralBuilding.PB_JitterPosition` _transformsselected (`self.JitterPosition`) (`self.RandomStream`)))
  ;[1 1 1] Jitter rotations based on probability
  (bind (_transformsunselected_3 _transformsselected_2) (`/Game/procedural_building/BPL_ProceduralBuilding.PB_SplitWithProbability` (`/Game/procedural_building/BPL_ProceduralBuilding.PB_Join` _transformsunselected_2 _transforms) (`self.RotateChance`) (`self.RandomStream`)))
  (bind _transforms_2 (`/Game/procedural_building/BPL_ProceduralBuilding.PB_JitterRotation` _transformsselected_2 (`self.JitterRotation`) (`self.RandomStream`)))
  ;[1 1 1] Construct Instanced Static Mesh from the result
  (`/Game/procedural_building/BPL_ProceduralBuilding.PB_AddInstancesToHISM` (`self.HierarchicalInstancedStaticMesh`) (`/Game/procedural_building/BPL_ProceduralBuilding.PB_Join` _transformsunselected_3 _transforms_2)))
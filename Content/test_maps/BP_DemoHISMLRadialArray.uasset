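; Demo Blueprint that builds a radial ring of a configurable mesh and materials as Hierarchical Instanced Static Mesh instances in its Construction Script.
; A chain of PB helper functions copies a default item around an arc, then randomly drops some copies by delete chance.
; Seeded probability splits jitter position, then rotation, on subsets of the survivors, rejoining each before all are added to the HISM.
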(fn `UserConstructionScript`
  ;[1 1 1] Set static mesh and materials
  (`StaticMeshComponent.SetStaticMesh` (`self.HierarchicalInstancedStaticMesh`) (`self.StaticMesh`))
  (for (_array_element _array_index) (`self.Materials`)
    (`PrimitiveComponent.SetMaterial` (`self.HierarchicalInstancedStaticMesh`) _array_index _array_element))
  ;[1 1 1] Delete some items based on chance
  (bind _transformsunselected (`/Game/procedural_building/BPL_ProceduralBuilding.PB_SplitWithProbability` (`/Game/procedural_building/BPL_ProceduralBuilding.PB_RadialArray` (`/Game/procedural_building/BPL_ProceduralBuilding.PB_DefaultItem`) (`self.ItemCount`) (`self.StartAngle`) (`self.EndAngle`) (`self.Radius`) (`self.CenterPoint`) (`self.RotateRoundCenterPoint`) (`self.Stepping`)) (`self.DeleteChance`) (`self.RandomStream`)))
  ;[1 1 1] Jitter transforms based on probability
  (bind (_transformsunselected_2 _transformsselected) (`/Game/procedural_building/BPL_ProceduralBuilding.PB_SplitWithProbability` _transformsunselected (`self.JitterChance`) (`self.RandomStream`)))
  (bind _transforms (`/Game/procedural_building/BPL_ProceduralBuilding.PB_JitterPosition` _transformsselected (`self.JitterPosition`) (`self.RandomStream`)))
  ;[1 1 1] Jitter rotations based on probability
  (bind (_transformsunselected_3 _transformsselected_2) (`/Game/procedural_building/BPL_ProceduralBuilding.PB_SplitWithProbability` (`/Game/procedural_building/BPL_ProceduralBuilding.PB_Join` _transformsunselected_2 _transforms) (`self.RotateChance`) (`self.RandomStream`)))
  (bind _transforms_2 (`/Game/procedural_building/BPL_ProceduralBuilding.PB_JitterRotation` _transformsselected_2 (`self.JitterRotation`) (`self.RandomStream`)))
  ;[1 1 1] Construct Instanced Static Mesh from the result
  (`/Game/procedural_building/BPL_ProceduralBuilding.PB_AddInstancesToHISM` (`self.HierarchicalInstancedStaticMesh`) (`/Game/procedural_building/BPL_ProceduralBuilding.PB_Join` _transformsunselected_3 _transforms_2)))